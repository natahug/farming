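; Game mode for a 360 video demo that switches the clip playing on a video sphere in response to menu button clicks.
; Initialize stores the sphere, menu and pawn, plays clip 1 from the Clips map and binds to the menu's click event.
; PlayClip looks up the clicked ID, then ChangeClip fades the pawn to black, waits the fade duration, swaps the video and fades in.
; VideoFinished is an empty stub.
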(event Custom|Play%20Clip
  (params (id :type Integer))
  (bind _clips (Variables|Default|GetClips))
  (bind (_value _returnvalue) (Utilities|Map|Find _clips id))
  ;[1 1 1] Function Binded to the OnButtonClick Event from the Menu... Plays the clip associated with the id via the map variable Clips... Current implementation fades the pawn down before performing the video switch
  (if _returnvalue
    (|ChangeClip _value)))

(fn ConstructionScript)

(fn Initialize
  (params (VideoSphere :type Video%20Sphere%20Object%20Reference) (Menu :type A%20360%20Video%20Demo%20UI%20Object%20Reference) (Pawn :type A%20GO%20Pawn%20Object%20Reference))
  ;[1 1 1] Initialize the variablesfor the Gamemode (Green) .Then play the first clip in the map (yellow). Then bind the Play Clip function the the OnButtonClick event from the menu (Blue).
  (Variables|Default|SetVideoSphere VideoSphere)
  (Variables|Default|SetMenu Menu)
  (Variables|Default|SetPawn Pawn)
  (Default|PlayClip (Variables|Default|GetVideoSphere) (.Value (Utilities|Map|Find (Variables|Default|GetClips) 1)))
  (EventDispatchers|BindEventtoOnButtonClicked (Variables|Default|GetMenu) (EventDispatchers|CreateEvent :!event Custom|Play%20Clip)))

(fn VideoFinished
  (params (clip%20id :type Integer)))