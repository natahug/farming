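; Game mode for a 360 video demo that moves the viewer between location clips chosen from a menu.
; Initialize stores the video sphere, menu and pawn, builds a clip-ID-to-location index, then plays the start clip.
; PlayClip fades the pawn's view around each clip switch and rebuilds the menu from a location adjacency map.
; That map changes at runtime, adding or removing the Intro option at Street depending on visited locations.
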(event Custom|Play%20Clip
  (params (id :type Integer))
  (bind (_succed _clip _location) (|FindClip id))
  (bind _pawn (Variables|Default|GetPawn))
  ;[1 1 1] Did not find location or clip
  (if _succed
    (|ModifyIntroDisplayinStreet _location)
    (Default|FadetoBlack _pawn)
    (bind _duration (Default|GetFadeDuration _pawn))
    (Utilities|FlowControl|Delay _duration)
    (Default|PlayClip (Variables|Default|GetVideoSphere) _clip)
    (bind _tmpclips (|Locationtonextclips _location))
    (Default|GenerateMenu (Variables|Default|GetMenu) _tmpclips)
    (Default|Fadein (Variables|Default|GetPawn))))

(fn ConstructionScript)

(fn Initialize
  (params (VideoSphere :type Video%20Sphere%20Object%20Reference) (Menu :type A%20360%20Video%20Demo%20UI%202%20Object%20Reference) (Pawn :type A%20GO%20Pawn%20Object%20Reference))
  ;[1 1 1] Init variables
  (Variables|Default|SetVideoSphere VideoSphere)
  (Variables|Default|SetMenu Menu)
  (Variables|Default|SetPawn Pawn)
  (CallFunction|ConstructReverseClipLocationIndex)
  (EventDispatchers|BindEventtoOnButtonClicked (Variables|Default|GetMenu) (EventDispatchers|CreateEvent :!event Custom|Play%20Clip))
  (Default|PlayClip (Variables|Default|GetVideoSphere) (.Value (Utilities|Map|Find (Variables|Default|GetClips) (LocalVariables|GetStart%20Location%20))))
  (bind _tmpclips (|Locationtonextclips_2 (LocalVariables|GetStart%20Location%20)))
  (Default|GenerateMenu (Variables|Default|GetMenu) _tmpclips))

(fn VideoFinished
  (params (clip%20id :type Integer)))

(fn ConstructReverseClipLocationIndex
  ;[1 1 1] For each location find the associated clip... The relationship between clip and location must be a bijection
  (bind _keys (Utilities|Map|Keys (Variables|Default|GetClips)))
  (for _array_element _keys
    (if (.ReturnValue (Utilities|Map|Find (Variables|Default|GetidtoLocation) (.id (Utilities|Struct|BreakClip (.Value (Utilities|Map|Find (Variables|Default|GetClips) _array_element))))))
      (Development|PrintString "Already seen a clip with that ID")
      (else
        (Utilities|Map|Add (Variables|Default|GetidtoLocation) (.id (Utilities|Struct|BreakClip (.Value (Utilities|Map|Find (Variables|Default|GetClips) _array_element)))) _array_element)))))